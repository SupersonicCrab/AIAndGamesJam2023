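; Player character Blueprint that takes its turn in a turn-based game run by GM_AIAndGamesJam2023.
; BeginPlay caches the game mode, and PerformTurn waits briefly before triggering the first ability in its ability component.
; When that component reports the ability finished, the character notifies the game mode that its turn is over.
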(event OnAbilityFinished(BPC_AbilityComponent)
  (params (Ability :type BP%20Ability%20Object%20Reference))
  (Default|OnTurnFinished (Variables|Default|GetGame%20Mode) self))

(event EventBeginPlay
  (bind _asgm_aiand_games_jam_2023 (Utilities|Casting|CastToGM_AIAndGamesJam2023 (Game|GetGameMode)))
  (Variables|Default|SetGame%20Mode _asgm_aiand_games_jam_2023))

(event EventPerformTurn
  (Utilities|FlowControl|Delay 0.666667)
  (Default|PerformAbility (Variables|Default|GetBPC_AbilityComponent) (Utilities|Array|Get(acopy) (Variables|/Game/Gameplay/GameObjects/Abilities/BPC_AbilityComponent.BPC_AbilityComponent_C|GetAbilites (Variables|Default|GetBPC_AbilityComponent)))))

(fn ConstructionScript)