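; Player controller for a turn-based game that handles mouse-driven movement and attacks for BP_PlayerCharacter.
; On possess it adds the HUD, caches the pawn's attack and movement components, and selects the first attack after a one-tick delay.
; During the player's turn, cursor traces on separate channels drive clicks on enabled BP_Compass bearings to move, an ability press to attack, and per-tick previews of the selected attack.
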(event EventTick
  (params (DeltaSeconds :type Float%20%28single-precision%29))
  (if (Variables|/Game/Gameplay/Players/BP_PlayerCharacter.BP_PlayerCharacter_C|GetbPlayersTurn (Variables|Default|GetPlayerCharacter))
    (bind _selectedattack (Variables|Default|GetSelectedAttack)
      (:then
        (Default|PreviewAttack (Variables|Default|GetAttackComponent) _selectedattack (.Location (Collision|BreakHitResult (.HitResult (Game|Player|GetHitResultUnderCursorbyChannel "TraceTypeQuery3" true))))))
      (:else))))

(event EventPossess
  (params (PossessedPawn :type Pawn%20Object%20Reference))
  (bind _self self)
  (Variables|Default|SetbShowMouseCursor true)
  (Utilities|FlowControl|Sequence
    (:then_0
      (bind _returnvalue (UserInterface|CreateWidget "/Game/UI/Widgets/WBP_HUD.WBP_HUD_C" _self))
      (UserInterface|Viewport|AddtoViewport _returnvalue 0)
      (Input|SetInputModeGameandUI _self 0 "DoNotLock" true false))
    (:then_1
      (bind _asbp_player_character (Utilities|Casting|CastToBP_PlayerCharacter (Pawn|GetControlledPawn)))
      (Variables|Default|SetPlayerCharacter _asbp_player_character)
      (Variables|Default|SetAttackComponent (Variables|/Game/Gameplay/Players/BP_PlayerCharacter.BP_PlayerCharacter_C|GetBPC_AttackComponent _asbp_player_character))
      (Variables|Default|SetMovementComponent (Variables|/Game/Gameplay/Players/BP_PlayerCharacter.BP_PlayerCharacter_C|GetBPC_MovementComponent _asbp_player_character))
      (Utilities|FlowControl|DelayUntilNextTick)
      (Variables|Default|SetSelectedAttack (Utilities|Array|Get(acopy) (Variables|/Game/Gameplay/GameObjects/Abilities/BPC_AttackComponent.BPC_AttackComponent_C|GetAttacks (Variables|Default|GetAttackComponent)))))))

(event Input|ActionEvents|InputActionAbility
  (params (Key :type Key%20Structure :default "None"))
  (:Pressed
    (if (Variables|/Game/Gameplay/Players/BP_PlayerCharacter.BP_PlayerCharacter_C|GetbPlayersTurn (Variables|Default|GetPlayerCharacter))
      (bind _selectedattack (Variables|Default|GetSelectedAttack)
        (:then
          (Default|PerformAttack (Variables|Default|GetAttackComponent) _selectedattack (.Location (Collision|BreakHitResult (.HitResult (Game|Player|GetHitResultUnderCursorbyChannel "TraceTypeQuery3" true))))))
        (:else)))))

(event Input|ActionEvents|InputActionMove
  (params (Key :type Key%20Structure :default "None"))
  (bind _hitresult (Game|Player|GetHitResultUnderCursorbyChannel "TraceTypeQuery4" true))
  (bind (_bblockinghit _binitialoverlap _time _distance _location _impactpoint _normal _impactnormal _physmat _hitactor _hitcomponent) (Collision|BreakHitResult _hitresult))
  (:Released
    (if (Variables|/Game/Gameplay/Players/BP_PlayerCharacter.BP_PlayerCharacter_C|GetbPlayersTurn (Variables|Default|GetPlayerCharacter))
      (bind _asbp_compass (Utilities|Casting|CastToBP_Compass _hitactor))
      (bind _asstatic_mesh_component (Utilities|Casting|CastToStaticMeshComponent _hitcomponent))
      (bind _bearing (Default|GetBearingfromMesh _asbp_compass _asstatic_mesh_component))
      (if (Utilities|Enum|NotEqual(Enum) _bearing "NewEnumerator16")
        (if (Default|IsBearingEnabled _asbp_compass _bearing)
          (Default|PerformMovementAbility (Variables|Default|GetMovementComponent) _location))))))

(fn ConstructionScript)