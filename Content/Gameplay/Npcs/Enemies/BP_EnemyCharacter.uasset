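; Turn-based enemy character that acts when PerformTurn runs and reports back to the game mode when finished.
; It performs a random valid attack from its attack component, otherwise steps toward a player visible by capsule trace, or wanders.
; Movement picks from enabled compass bearings that pass a death-fall check.
; Attack or movement completion ends the turn; death drops attacks, releases any active turn and removes it from play.
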(event OnMovementAbilityFinished(BPC_MovementComponent)
  (params (MovementAbility :type BP%20Movement%20Ability%20Object%20Reference))
  (CallFunction|EndTurn))

(event OnDeath(BPC_HealthComponent)
  (Default|DropAllAttacks (Variables|Default|GetBPC_AttackComponent))
  (Utilities|FlowControl|Sequence
    (:then_0
      (if (Variables|Default|GetbEnemiesTurn)
        (Default|OnTurnFinished (Variables|Default|GetGameMode) self)))
    (:then_1
      (Utilities|Array|RemoveItem (Variables|/Game/Gameplay/Systems/GM_AIAndGamesJam2023.GM_AIAndGamesJam2023_C|GetTurnActors (Variables|Default|GetGameMode)) self)
      (Development|PrintString "Enemy died" true true "(R=1.000000,G=0.000000,B=0.000000,A=1.000000)")
      (Actor|DestroyActor))))

(event OnTakeDamage(BPC_HealthComponent)
  (params (DamageAmount :type Integer))
  (Development|PrintString (Utilities|String|Append "Remaining enemy health: " (Utilities|String|ToString(Integer) (Variables|/Game/Gameplay/GameObjects/BPC_HealthComponent.BPC_HealthComponent_C|GetHealth (Variables|Default|GetBPC_HealthComponent)))) true true "(R=1.000000,G=0.000000,B=0.000000,A=1.000000)"))

(event OnAttackFinished(BPC_AttackComponent)
  (params (Attack :type BP%20Attack%20Ability%20Object%20Reference))
  (CallFunction|EndTurn))

(event EventBeginPlay
  (bind _asgm_aiand_games_jam_2023 (Utilities|Casting|CastToGM_AIAndGamesJam2023 (Game|GetGameMode)))
  (Variables|Default|SetGameMode _asgm_aiand_games_jam_2023)
  (Variables|Default|SetPlayerCharacter (Game|GetPlayerCharacter 0)))

(event EventPerformTurn
  (Variables|Default|SetbEnemiesTurn true)
  (if (> (Variables|/Game/Gameplay/GameObjects/BPC_HealthComponent.BPC_HealthComponent_C|GetHealth (Variables|Default|GetBPC_HealthComponent)) 0)
    (bind _validattacks (CallFunction|GetValidAttacks))
    (if (Utilities|Array|IsNotEmpty _validattacks)
      (bind _target (Default|GetEnemyTarget (.OutItem (Utilities|Array|Random _validattacks))))
      (Default|PerformAttack (Variables|Default|GetBPC_AttackComponent) (.OutItem (Utilities|Array|Random _validattacks)) (Transformation|GetActorLocation _target))
      (else
        (bind _bplayervisible (CallFunction|IsPlayerVisible))
        (if _bplayervisible
          (Development|PrintString "move towards player")
          (CallFunction|MoveTowardsPlayer)
          (else
            (Development|PrintString "wander")
            (CallFunction|WanderAroundMap)))))))

(fn ConstructionScript
  (bind _asbp_compass (Utilities|Casting|CastToBP_Compass (Variables|/Script/Engine.ChildActorComponent|GetChildActor (Variables|Default|GetCompass))))
  (Variables|Default|SetCompassRef _asbp_compass))

(fn GetValidAttacks
  (for _array_element (Variables|/Game/Gameplay/GameObjects/Abilities/BPC_AttackComponent.BPC_AttackComponent_C|GetAttacks (Variables|Default|GetBPC_AttackComponent))
    (bind _target (Default|GetEnemyTarget _array_element))
    (Variables|/Game/Gameplay/GameObjects/Abilities/Attack/BP_AttackAbility.BP_AttackAbility_C|SetTargetLocation _array_element (Transformation|GetActorLocation _target))
    (bind _bcanperform (Default|CanPerformAttack _array_element))
    (if _bcanperform
      (Utilities|Array|Add (LocalVariables|GetTempAttacks) _array_element)))
  (return (LocalVariables|GetTempAttacks)))

(fn EndTurn
  (Variables|Default|SetbEnemiesTurn false)
  (Default|OnTurnFinished (Variables|Default|GetGameMode) self))

(fn IsPlayerVisible
  (bind _capsulecomponent (Variables|Collision|GetCapsuleComponent))
  (bind _outhit (Collision|CapsuleTraceByChannel (Transformation|GetActorLocation) (Transformation|GetActorLocation (Variables|Default|GetPlayerCharacter)) (Components|Capsule|GetScaledCapsuleRadius _capsulecomponent) (Variables|/Script/Engine.CapsuleComponent|GetCapsuleHalfHeight _capsulecomponent) "TraceTypeQuery1" false (Utilities|Array|MakeArray (Variables|Default|GetCompassRef)) "ForOneFrame"))
  (return (== (.HitActor (Collision|BreakHitResult _outhit)) (Variables|Default|GetPlayerCharacter))))

(fn GetSafeBearings
  (bind _compassref (Variables|Default|GetCompassRef))
  (bind _bearingtomesh (Variables|/Game/Gameplay/GameObjects/Compass/BP_Compass.BP_Compass_C|GetBearingToMesh _compassref))
  (bind _values (Utilities|Map|Values _bearingtomesh))
  (LocalVariables|SetBearingMeshs _values)
  (bind _keys (Utilities|Map|Keys _bearingtomesh))
  (for (_array_element _array_index) _keys
    (if (Default|IsBearingEnabled (Variables|Default|GetCompassRef) _array_element)
      (bind _bdeathfall (CallFunction|CheckDeathFall self (.Origin (Collision|GetComponentBounds (Utilities|Array|Get(acopy) (LocalVariables|GetBearingMeshs) _array_index))) -4e+02))
      (if (not _bdeathfall)
        (Utilities|Array|Add (LocalVariables|GetTempSafeBearings) (Utilities|Array|Get(acopy) (LocalVariables|GetBearingMeshs) _array_index)))))
  (return (LocalVariables|GetTempSafeBearings)))

(fn MoveTowardsPlayer
  (bind _safebearings (CallFunction|GetSafeBearings))
  (if (Utilities|Array|IsNotEmpty _safebearings)
    (for _array_element _safebearings
      (if (< (Math|Vector|Distance(Vector) (Transformation|GetActorLocation (Variables|Default|GetPlayerCharacter)) (.Origin (Collision|GetComponentBounds _array_element))) (LocalVariables|GetClosestBearingDistance))
        (LocalVariables|SetClosestBearing _array_element)
        (LocalVariables|SetClosestBearingDistance (Math|Vector|Distance(Vector) (Transformation|GetActorLocation (Variables|Default|GetPlayerCharacter)) (.Origin (Collision|GetComponentBounds _array_element))))))
    (bind _closestbearing (LocalVariables|GetClosestBearing)
      (:then
        (Default|PerformMovementAbility (Variables|Default|GetBPC_MovementComponent) (.Origin (Collision|GetComponentBounds _closestbearing))))
      (:else))
    (else
      (CallFunction|EndTurn))))

(fn WanderAroundMap
  (bind _safebearings (CallFunction|GetSafeBearings))
  (if (Utilities|Array|IsNotEmpty _safebearings)
    (Default|PerformMovementAbility (Variables|Default|GetBPC_MovementComponent) (.Origin (Collision|GetComponentBounds (.OutItem (Utilities|Array|Random _safebearings)))))
    (else
      (CallFunction|EndTurn))))