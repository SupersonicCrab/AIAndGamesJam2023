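; Game mode for the AI and Games Jam 2023 project that runs a turn-based loop over actors implementing BPI_TurnActor.
; On BeginPlay it gathers those actors, moves player characters to the front of the queue and starts the first turn a tick later.
; Each turn messages the front actor; OnTurnFinished rotates it to the back and starts the next, with a delay after enemy turns.
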(event Custom|OnTurnFinished
  (params (TurnActor :type Actor%20Object%20Reference))
  (Development|PrintString (Utilities|String|Append (Utilities|GetDisplayName TurnActor) " turn finished"))
  (CallFunction|MoveTurnActorBottom TurnActor)
  (if (Class|GameplayStatics|ObjectIsA TurnActor "/Game/Gameplay/Npcs/Enemies/BP_EnemyCharacter.BP_EnemyCharacter_C")
    (Utilities|FlowControl|Delay (Variables|Default|GetEnemyTurnDelay))
    (CallFunction|StartNextTurn)
    (else
      (CallFunction|StartNextTurn))))

(event EventBeginPlay
  (bind _outactors (Actor|GetAllActorswithInterface "/Game/Gameplay/Systems/BPI_TurnActor.BPI_TurnActor_C"))
  (Variables|Default|SetTurnActors _outactors)
  (CallFunction|SortPlayers)
  (Utilities|FlowControl|DelayUntilNextTick)
  (CallFunction|StartNextTurn))

(fn ConstructionScript)

(fn SortPlayers
  (for _array_element (Variables|Default|GetTurnActors)
    (bind _asbp_player_character (Utilities|Casting|CastToBP_PlayerCharacter _array_element))
    (CallFunction|MoveTurnActorTop _asbp_player_character)))

(fn StartNextTurn
  (bind _turnactors (Variables|Default|GetTurnActors))
  (bind _output (Utilities|Array|Get(acopy) _turnactors))
  (Development|PrintString (Utilities|String|Append (Utilities|GetDisplayName _output) " turn started"))
  (Class|BPITurnActor|PerformTurn(Message) _output))

(fn MoveTurnActorTop
  (params (TurnActor :type Actor%20Object%20Reference))
  (Utilities|Array|RemoveItem (Variables|Default|GetTurnActors) TurnActor)
  (Utilities|Array|Insert (Variables|Default|GetTurnActors) TurnActor))

(fn MoveTurnActorBottom
  (params (TurnActor :type Actor%20Object%20Reference))
  (Utilities|Array|RemoveItem (Variables|Default|GetTurnActors) TurnActor)
  (Utilities|Array|Add (Variables|Default|GetTurnActors) TurnActor))