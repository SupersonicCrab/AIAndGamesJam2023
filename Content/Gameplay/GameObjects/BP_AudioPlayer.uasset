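; BP_AudioPlayer is a game object that plays a randomly chosen sound from its Sounds array through its Audio component.
; On BeginPlay, if the array is not empty, it binds a handler to the component's OnAudioFinished event and calls PlayRandomAudio.
; PlayRandomAudio sets a random entry as the component's sound and plays it from the start.
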(event EventBeginPlay
  (if (Utilities|Array|IsNotEmpty (Variables|Default|GetSounds))
    (EventDispatchers|AssignOnAudioFinished (Variables|Default|GetAudio) (EventDispatchers|CreateEvent :!event PlayRandomAudio))
    (CallFunction|PlayRandomAudio)))

(fn ConstructionScript)

(fn PlayRandomAudio
  (Audio|Components|Audio|SetSound (Variables|Default|GetAudio) (.OutItem (Utilities|Array|Random (Variables|Default|GetSounds))))
  (Audio|Components|Audio|Play (Variables|Default|GetAudio) 0.0))