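; Actor component that manages its owner's attack abilities, from creation through preview and execution to drop and pickup.
; On BeginPlay it spawns the starting attack classes as owned actors and tracks them, appending or removing their disabled bearings on an optional Compass.
; Performing or previewing flattens the target to the owner's height and checks whether the attack can run.
; Finished abilities are relayed through an attack-finished dispatcher.
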(event Custom|OnAbilityFinished_Event
  (params (Ability :type BP%20Ability%20Object%20Reference))
  (Development|PrintString (Utilities|String|Append (Utilities|GetDisplayName (Components|GetOwner)) " finished ability " (Utilities|GetDisplayName Ability)))
  (Default|CallOnAttackFinished (stale Custom|PerformAttack Attack)))

(event Custom|PerformAttack
  (params (Attack :type BP%20Attack%20Ability%20Object%20Reference) (TargetLocation :type Vector))
  (bind (_x _y) (Math|Vector|BreakVector TargetLocation))
  (EventDispatchers|AssignOnAbilityFinished Attack (delegate Custom|OnAbilityFinished_Event))
  (Variables|/Game/Gameplay/GameObjects/Abilities/Attack/BP_AttackAbility.BP_AttackAbility_C|SetTargetLocation Attack (Math|Vector|MakeVector _x _y (.z (Transformation|GetActorLocation (Components|GetOwner)))))
  (bind _bcanperform (Default|CanPerformAttack Attack))
  (if _bcanperform
    (Development|PrintString (Utilities|String|Append (Utilities|GetDisplayName (Components|GetOwner)) " starting attack ability " (Utilities|GetDisplayName Attack)))
    (Default|PerformAbility Attack)))

(event EventBeginPlay
  (CallFunction|CreateAttacks (Variables|Default|GetStartingAttacks)))

(fn CreateAttacks
  (params (AbilityClasses :type Array%20of%20BP%20Attack%20Ability%20Class%20References))
  (for _array_element AbilityClasses
    (CallFunction|CreateAttack _array_element)))

(fn CreateAttack
  (params (Class :type BP%20Attack%20Ability%20Class%20Reference))
  (bind _returnvalue (Game|SpawnActorfromClass Class (Math|Transform|MakeTransform "0, 0, 0" "0, 0, 0" "1.000000,1.000000,1.000000") "Undefined" "MultiplyWithRoot" (Components|GetOwner) 0))
  (CallFunction|AddAttack _returnvalue))

(fn AddAttack
  (params (Attack :type BP%20Attack%20Ability%20Object%20Reference%20%28by%20ref%29))
  (Utilities|Array|Add (Variables|Default|GetAttacks) Attack)
  (Default|CallOnAttackAdded Attack)
  (bind _compass (Variables|Default|GetCompass)
    (:then
      (Utilities|Array|AppendArray (Variables|/Game/Gameplay/GameObjects/Compass/BP_Compass.BP_Compass_C|GetDisabledBearing _compass) (Variables|/Game/Gameplay/GameObjects/Abilities/Attack/BP_AttackAbility.BP_AttackAbility_C|GetDisabledBearings Attack))
      (Default|UpdateCompassBearings (Variables|Default|GetCompass)))
    (:else)))

(fn RemoveAttack
  (params (Attack :type BP%20Attack%20Ability%20Object%20Reference))
  (Utilities|Array|RemoveItem (Variables|Default|GetAttacks) Attack)
  (bind _compass (Variables|Default|GetCompass)
    (:then
      (for _array_element (Variables|/Game/Gameplay/GameObjects/Abilities/Attack/BP_AttackAbility.BP_AttackAbility_C|GetDisabledBearings Attack)
        (Utilities|Array|RemoveItem (Variables|/Game/Gameplay/GameObjects/Compass/BP_Compass.BP_Compass_C|GetDisabledBearing _compass) _array_element))
      (Default|UpdateCompassBearings (Variables|Default|GetCompass)))
    (:else)))

(fn DropAllAttacks
  (for _array_element (Variables|Default|GetAttacks)
    (CallFunction|DropAttack _array_element)))

(fn DropAttack
  (params (Attack :type BP%20Attack%20Ability%20Object%20Reference))
  (Default|OnDropped Attack (Transformation|GetActorLocation (Components|GetOwner)))
  (CallFunction|RemoveAttack Attack))

(fn PickupAttack
  (params (Attack :type BP%20Attack%20Ability%20Object%20Reference))
  (Default|OnPickedUp Attack)
  (CallFunction|AddAttack Attack))

(fn PreviewAttack
  (params (Attack :type BP%20Attack%20Ability%20Object%20Reference) (TargetLocation :type Vector))
  (Variables|/Game/Gameplay/GameObjects/Abilities/Attack/BP_AttackAbility.BP_AttackAbility_C|SetTargetLocation Attack (Math|Vector|MakeVector (.x TargetLocation) (.y TargetLocation) (.z (Transformation|GetActorLocation (Components|GetOwner)))))
  (bind _bcanperform (Default|CanPerformAttack Attack))
  (if _bcanperform
    (Default|PreviewAttack Attack)
    (else
      (Default|EnableAttackPreview Attack false))))