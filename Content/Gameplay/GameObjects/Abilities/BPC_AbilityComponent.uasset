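; BPC_AbilityComponent is an actor component that creates and runs its owner's abilities.
; On BeginPlay it spawns each starting ability class as an actor owned by the component's owner, sorting movement abilities and other abilities into separate arrays.
; PerformAbility binds to the given ability's finished event and starts it, then the component relays completion through its own OnAbilityFinished dispatcher, printing debug messages at start and finish.
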(event Custom|OnAbilityFinished_Event
  (params (Ability :type BP%20Ability%20Object%20Reference))
  (Development|PrintString (Utilities|String|Append (Utilities|GetDisplayName (Components|GetOwner)) " finished ability " (Utilities|GetDisplayName Ability)))
  (Default|CallOnAbilityFinished Ability))

(event Custom|PerformAbility
  (params (Ability :type BP%20Ability%20Object%20Reference))
  (Development|PrintString (Utilities|String|Append (Utilities|GetDisplayName (Components|GetOwner)) " starting ability " (Utilities|GetDisplayName Ability)))
  (EventDispatchers|AssignOnAbilityFinished Ability (delegate Custom|OnAbilityFinished_Event))
  (Default|PerformAbility Ability))

(event EventBeginPlay
  (CallFunction|CreateAbilities (Variables|Default|GetStartingAbilities)))

(fn CreateAbilities
  (params (AbilityClasses :type Array%20of%20BP%20Ability%20Class%20References))
  (for _array_element AbilityClasses
    (CallFunction|CreateAbility _array_element)))

(fn CreateAbility
  (params (Class :type BP%20Ability%20Class%20Reference))
  (bind _returnvalue (Game|SpawnActorfromClass Class (Math|Transform|MakeTransform "0, 0, 0" "0, 0, 0" "1.000000,1.000000,1.000000") "Undefined" "MultiplyWithRoot" (Components|GetOwner) 0))
  (if (Class|GameplayStatics|ObjectIsA _returnvalue "/Game/Gameplay/GameObjects/Abilities/Movement/BP_MovementAbility.BP_MovementAbility_C")
    (Utilities|Array|Add (Variables|Default|GetMovementAbilities) 0)
    (elif (Class|GameplayStatics|ObjectIsA _returnvalue "/Game/Gameplay/GameObjects/Abilities/BP_Ability.BP_Ability_C")
      (Utilities|Array|Add (Variables|Default|GetAbilities) _returnvalue))))