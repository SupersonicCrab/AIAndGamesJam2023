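; BP_Ability is a base ability actor that also exists in the world as a pickup.
; PerformAbility is an empty hook, and FinishAbility fires the OnAbilityFinished dispatcher.
; OnDropped teleports the actor to the drop location, shows the Sphere and enables query-only pickup collision.
; OnPickedUp hides the Sphere and disables that collision, so the same actor persists between dropped and carried states.
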(fn ConstructionScript)

(fn PerformAbility)

(fn FinishAbility
  (Default|CallOnAbilityFinished self))

(fn OnDropped
  (params (DropLocation :type Vector))
  (Transformation|SetActorLocation DropLocation false true)
  (Rendering|SetVisibility (Variables|Default|GetSphere) true true)
  (Collision|SetCollisionEnabled (Variables|Default|GetPickupCollision) "QueryOnly"))

(fn OnPickedUp
  (Rendering|SetVisibility (Variables|Default|GetSphere) false true)
  (Collision|SetCollisionEnabled (Variables|Default|GetPickupCollision) "NoCollision"))