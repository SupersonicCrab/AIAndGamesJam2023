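; Frog animal attack ability that moves its owner to the far side of a Character it hits.
; It overrides AffectTarget, running the parent effect before casting the hit actor to Character.
; The owner is then placed beyond the target along the line between them, at the same distance it started from, mirroring its position.
; The move is an instant SetActorLocation without sweep, so nothing in between blocks it.
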(event EventBeginPlay
  (|CallParentFunction) ; This node is disabled and will not be called.\nDrag off pins to build functionality.
)

(event Collision|EventActorBeginOverlap
  (params (OtherActor :type Actor%20Object%20Reference))
  (|CallParentFunction OtherActor) ; This node is disabled and will not be called.\nDrag off pins to build functionality.
)

(event EventTick
  (params (DeltaSeconds :type Float%20%28single-precision%29))
  (|CallParentFunction DeltaSeconds) ; This node is disabled and will not be called.\nDrag off pins to build functionality.
)

(fn ConstructionScript
  (|CallParentFunction))

(fn AffectTarget
  (params (HitActor :type Actor%20Object%20Reference) (ImpactLocation :type Vector :default "0, 0, 0"))
  (bind _returnvalue (Components|GetOwner))
  (bind _returnvalue_2 (Transformation|GetActorLocation HitActor))
  (bind _returnvalue_3 (Transformation|GetActorLocation _returnvalue))
  (|CallParentFunction HitActor ImpactLocation)
  (Utilities|Casting|CastToCharacter HitActor)
  (Transformation|SetActorLocation (Components|GetOwner) (+ _returnvalue_2 (* (Math|Vector|GetForwardVector (Math|Rotator|FindLookatRotation _returnvalue_3 _returnvalue_2)) (Math|Vector|Distance(Vector) _returnvalue_2 _returnvalue_3))) false false))