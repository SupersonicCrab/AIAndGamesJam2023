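; BP_AOE_Anglerfish is the Anglerfish's area-of-effect attack ability, which drags characters caught in its sphere toward the center.
; CanPerformAttack passes only when the parent check succeeds and the sphere overlap finds at least one result.
; AffectTarget runs the parent effect, then reuses PushCharacter as a pull, aiming each hit Character at SphereCenter over its exact distance to it, with enemy collision enabled.
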(fn ConstructionScript
  (|CallParentFunction))

(fn AffectTarget
  (params (HitActor :type Actor%20Object%20Reference) (ImpactLocation :type Vector :default "0, 0, 0"))
  (bind _returnvalue (Transformation|GetActorLocation HitActor))
  (bind _spherecenter (Variables|Default|GetSphereCenter))
  (|CallParentFunction HitActor ImpactLocation)
  (bind _ascharacter (Utilities|Casting|CastToCharacter HitActor))
  (CallFunction|PushCharacter _ascharacter (Math|Vector|GetForwardVector (Math|Rotator|FindLookatRotation _returnvalue _spherecenter)) (Math|Vector|Distance(Vector) _returnvalue _spherecenter) true 5.0))

(fn CanPerformAttack
  (bind _bcanperform (|CallParentFunction))
  (if _bcanperform
    (bind _outactors (CallFunction|GetSphereOverlapResults))
    (return (not (Utilities|Array|IsEmpty _outactors)))
    (else
      (return false))))