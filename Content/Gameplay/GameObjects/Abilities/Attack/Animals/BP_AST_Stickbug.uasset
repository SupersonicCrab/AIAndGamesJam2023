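; Stickbug animal attack ability that knocks attacker and target apart when it affects a target.
; AffectTarget runs the inherited effect, then pushes the hit Character away from the owner along the owner-to-target direction.
; The owning Character is pushed the same distance backward using a negative distance on that direction, with enemy collision enabled for both pushes.
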(event EventBeginPlay
  (|CallParentFunction) ; This node is disabled and will not be called.\nDrag off pins to build functionality.
)

(event Collision|EventActorBeginOverlap
  (params (OtherActor :type Actor%20Object%20Reference))
  (|CallParentFunction OtherActor) ; This node is disabled and will not be called.\nDrag off pins to build functionality.
)

(event EventTick
  (params (DeltaSeconds :type Float%20%28single-precision%29))
  (|CallParentFunction DeltaSeconds) ; This node is disabled and will not be called.\nDrag off pins to build functionality.
)

(fn ConstructionScript
  (|CallParentFunction))

(fn AffectTarget
  (params (HitActor :type Actor%20Object%20Reference) (ImpactLocation :type Vector :default "0, 0, 0"))
  (bind _returnvalue (Transformation|GetActorLocation HitActor))
  (bind _returnvalue_2 (Components|GetOwner))
  (bind _returnvalue_3 (Transformation|GetActorLocation _returnvalue_2))
  (bind _returnvalue_4 (Math|Rotator|FindLookatRotation _returnvalue_3 _returnvalue))
  (bind _returnvalue_5 (Math|Vector|GetForwardVector _returnvalue_4))
  (|CallParentFunction HitActor ImpactLocation)
  (Utilities|FlowControl|Sequence
    (:then_0
      (bind _ascharacter (Utilities|Casting|CastToCharacter HitActor))
      (CallFunction|PushCharacter _ascharacter _returnvalue_5 (Math|Float|Absolute(Float) 1e+02) true 5e+01))
    (:then_1
      (bind _ascharacter_2 (Utilities|Casting|CastToCharacter (Components|GetOwner)))
      (CallFunction|PushCharacter _ascharacter_2 _returnvalue_5 (Math|Float|MakeLiteralFloat -1e+02) true 5e+01))))