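; BP_AoE_Moth is the area-of-effect attack for the Moth animal ability, adding knockback to the targets it hits.
; Its AffectTarget override runs the parent effect, then pushes any Character target a short fixed distance directly away from the effect's owner, with enemy collision enabled.
; The event graph and construction script add no logic, so all other behavior comes from the parent class.
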(event EventBeginPlay
  (|CallParentFunction) ; This node is disabled and will not be called.\nDrag off pins to build functionality.
)

(event Collision|EventActorBeginOverlap
  (params (OtherActor :type Actor%20Object%20Reference))
  (|CallParentFunction OtherActor) ; This node is disabled and will not be called.\nDrag off pins to build functionality.
)

(event EventTick
  (params (DeltaSeconds :type Float%20%28single-precision%29))
  (|CallParentFunction DeltaSeconds) ; This node is disabled and will not be called.\nDrag off pins to build functionality.
)

(fn ConstructionScript
  (|CallParentFunction))

(fn AffectTarget
  (params (HitActor :type Actor%20Object%20Reference) (ImpactLocation :type Vector :default "0, 0, 0"))
  (|CallParentFunction HitActor ImpactLocation)
  (bind _ascharacter (Utilities|Casting|CastToCharacter HitActor))
  (CallFunction|PushCharacter _ascharacter (Math|Vector|GetForwardVector (Math|Rotator|FindLookatRotation (Transformation|GetActorLocation (Components|GetOwner)) (Transformation|GetActorLocation HitActor))) 1.5e+02 true 5e+01))