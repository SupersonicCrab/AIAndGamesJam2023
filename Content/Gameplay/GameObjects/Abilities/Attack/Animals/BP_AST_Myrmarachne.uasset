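; Myrmarachne animal attack ability that repositions itself and the actor it hits, in a swap-like move.
; AffectTarget runs the parent effect, then caches the hit actor's location and the owner's location.
; It teleports the ability actor itself, not the owner, to the target's old position, then moves the target to the owner's position without sweeping.
; The event graph holds only disabled stubs.
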(event EventBeginPlay
  (|CallParentFunction) ; This node is disabled and will not be called.\nDrag off pins to build functionality.
)

(event Collision|EventActorBeginOverlap
  (params (OtherActor :type Actor%20Object%20Reference))
  (|CallParentFunction OtherActor) ; This node is disabled and will not be called.\nDrag off pins to build functionality.
)

(event EventTick
  (params (DeltaSeconds :type Float%20%28single-precision%29))
  (|CallParentFunction DeltaSeconds) ; This node is disabled and will not be called.\nDrag off pins to build functionality.
)

(fn ConstructionScript
  (|CallParentFunction))

(fn AffectTarget
  (params (HitActor :type Actor%20Object%20Reference) (ImpactLocation :type Vector :default "0, 0, 0"))
  (|CallParentFunction HitActor ImpactLocation)
  (bind _output_get (LocalVariables|SetEnemyPosition (Transformation|GetActorLocation HitActor)))
  (bind _output_get_2 (LocalVariables|SetSelfPosition (Transformation|GetActorLocation (Components|GetOwner))))
  (Transformation|SetActorLocation _output_get false true)
  (Transformation|SetActorLocation HitActor _output_get_2 false false))