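; Area-of-effect attack ability for the Snapping Turtle animal that heals its owner when it affects a target.
; It overrides AffectTarget, runs the parent behavior, then finds the owner's BPC_HealthComponent and heals a tenth of that owner's max health on each call.
; All other behavior comes from the parent class, as the event graph holds only disabled stubs.
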(event EventBeginPlay
  (|CallParentFunction) ; This node is disabled and will not be called.\nDrag off pins to build functionality.
)

(event Collision|EventActorBeginOverlap
  (params (OtherActor :type Actor%20Object%20Reference))
  (|CallParentFunction OtherActor) ; This node is disabled and will not be called.\nDrag off pins to build functionality.
)

(event EventTick
  (params (DeltaSeconds :type Float%20%28single-precision%29))
  (|CallParentFunction DeltaSeconds) ; This node is disabled and will not be called.\nDrag off pins to build functionality.
)

(fn ConstructionScript
  (|CallParentFunction))

(fn AffectTarget
  (params (HitActor :type Actor%20Object%20Reference) (ImpactLocation :type Vector :default "0, 0, 0"))
  (bind _returnvalue (Components|GetOwner))
  (bind _returnvalue_2 (Actor|GetComponentbyClass _returnvalue "/Game/Gameplay/GameObjects/BPC_HealthComponent.BPC_HealthComponent_C"))
  (|CallParentFunction HitActor ImpactLocation)
  (Default|Heal _returnvalue_2 (/ (Variables|/Game/Gameplay/GameObjects/BPC_HealthComponent.BPC_HealthComponent_C|GetMaxHealth _returnvalue_2) 10)))