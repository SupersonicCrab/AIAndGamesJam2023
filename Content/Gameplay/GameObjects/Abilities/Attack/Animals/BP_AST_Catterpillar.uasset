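; BP_AST_Catterpillar is an animal attack ability that lunges its owning character toward the point of impact.
; Its AffectTarget override pushes the owner along the look-at direction to the impact location, over the distance to that point, with enemy collision enabled.
; It then calls the parent AffectTarget; if the owner is not a Character, it stops before both the push and that call.
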(event EventBeginPlay
  (|CallParentFunction) ; This node is disabled and will not be called.\nDrag off pins to build functionality.
)

(event Collision|EventActorBeginOverlap
  (params (OtherActor :type Actor%20Object%20Reference))
  (|CallParentFunction OtherActor) ; This node is disabled and will not be called.\nDrag off pins to build functionality.
)

(event EventTick
  (params (DeltaSeconds :type Float%20%28single-precision%29))
  (|CallParentFunction DeltaSeconds) ; This node is disabled and will not be called.\nDrag off pins to build functionality.
)

(fn ConstructionScript
  (|CallParentFunction))

(fn AffectTarget
  (params (HitActor :type Actor%20Object%20Reference) (ImpactLocation :type Vector :default "0, 0, 0"))
  (bind _returnvalue (Components|GetOwner))
  (bind _returnvalue_2 (Transformation|GetActorLocation _returnvalue))
  (bind _ascharacter (Utilities|Casting|CastToCharacter _returnvalue))
  (CallFunction|PushCharacter _ascharacter (Math|Vector|GetForwardVector (Math|Rotator|FindLookatRotation _returnvalue_2 ImpactLocation)) (Math|Float|Absolute(Float) (Math|Vector|Distance(Vector) ImpactLocation _returnvalue_2)) true 5e+01)
  (|CallParentFunction HitActor ImpactLocation))