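; BP_AttackAbility is a base attack ability pickup, with placeholder perform, range and preview functions that suggest child Blueprints supply the attack.
; Player overlap passes it to the character's attack component, and BeginPlay caches a BP_Compass from the owner's first child actor.
; It targets player 0, toggles preview off on finish, and can heal that player before destroying itself.
; When dropped near a BP_DeathZone, it expires after a short lifespan.
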(event OnComponentBeginOverlap(PickupCollision)
  (params (OverlappedComponent :type Primitive%20Component%20Object%20Reference) (OtherActor :type Actor%20Object%20Reference) (OtherComp :type Primitive%20Component%20Object%20Reference) (OtherBodyIndex :type Integer) (bFromSweep :type Boolean) (SweepResult :type Hit%20Result%20Structure%20%28by%20ref%29))
  (bind _asbp_player_character (Utilities|Casting|CastToBP_PlayerCharacter OtherActor))
  (Default|PickupAttack (Variables|/Game/Gameplay/Players/BP_PlayerCharacter.BP_PlayerCharacter_C|GetBPC_AttackComponent _asbp_player_character) self))

(event EventBeginPlay
  (|CallParentFunction)
  (bind _asbp_compass (Utilities|Casting|CastToBP_Compass (Utilities|Array|Get(acopy) (Actor|GetAllChildActors (Components|GetOwner) true))))
  (Variables|Default|SetOwningCompass _asbp_compass))

(fn ConstructionScript
  (|CallParentFunction))

(fn PerformAbility)

(fn CanPerformAttack
  (return false))

(fn GetEnemyTarget
  (bind _returnvalue (Game|GetPlayerCharacter 0))
  (Utilities|IsValid _returnvalue
    (:Is%20Valid
      (return _returnvalue))
    (:Is%20Not%20Valid
      (return 0))))

(fn OnDropped
  (params (DropLocation :type Vector :default "0, 0, 0"))
  (|CallParentFunction DropLocation)
  (bind _returnvalue (Collision|SphereOverlapActors DropLocation 1e+02 (Utilities|Array|MakeArray "ObjectTypeQuery2") "/Game/Gameplay/Systems/BP_DeathZone.BP_DeathZone_C"))
  (if _returnvalue
    (Actor|SetLifeSpan 1.0)))

(fn EnableAttackPreview
  (params (bEnabled :type Boolean)))

(fn PreviewAttack
  (CallFunction|EnableAttackPreview true))

(fn FinishAbility
  (|CallParentFunction)
  (CallFunction|EnableAttackPreview false))

(fn HealPlayer
  (Default|Heal (Actor|GetComponentbyClass (Game|GetPlayerCharacter 0) "/Game/Gameplay/GameObjects/BPC_HealthComponent.BPC_HealthComponent_C") (Variables|Default|GetDuplicatePickupHealAmount))
  (Actor|DestroyActor))

(fn GetMinRange
  (return 0.0))