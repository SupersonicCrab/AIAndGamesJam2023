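; Area-of-effect attack ability that affects every pawn within AOERadius of a targeted point, then finishes.
; The sphere centers on the inherited trace's blocking hit, or TargetLocation if nothing blocks, and ignores the owner and OwningCompass.
; The attack preview extends the parent's by moving AOETargetPreview to the stored SphereCenter, scaling it to the radius and toggling its visibility.
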(fn ConstructionScript
  (|CallParentFunction))

(fn PerformAbility
  (bind _outactors (CallFunction|GetSphereOverlapResults))
  (for _array_element _outactors
    (CallFunction|AffectTarget _array_element "0, 0, 0"))
  (CallFunction|FinishAbility))

(fn GetSphereOverlapResults
  (bind (_outhit _bblockinghit) (CallFunction|GetSphereTraceResults))
  (bind _output_get (Variables|Default|SetSphereCenter (Math|Vector|SelectVector (.Location (Collision|BreakHitResult _outhit)) (Variables|Default|GetTargetLocation) _bblockinghit)))
  (bind _outactors (Collision|SphereOverlapActors _output_get (Variables|Default|GetAOERadius) (Utilities|Array|MakeArray "ObjectTypeQuery3") 0 (Utilities|Array|MakeArray (Variables|Default|GetOwningCompass) (Components|GetOwner))))
  (return _outactors))

(fn PreviewAttack
  (|CallParentFunction)
  (Transformation|SetWorldLocation (Variables|Default|GetAOETargetPreview) (Variables|Default|GetSphereCenter) false true)
  (Transformation|SetRelativeScale3D (Variables|Default|GetAOETargetPreview) (Math|Conversions|ToVector(Float) (/ (Variables|Default|GetAOERadius) 1e+02))))

(fn EnableAttackPreview
  (params (bEnabled :type Boolean))
  (|CallParentFunction bEnabled)
  (Rendering|SetVisibility (Variables|Default|GetAOETargetPreview) bEnabled false))