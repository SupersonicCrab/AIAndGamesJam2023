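; Single-target attack ability that damages one actor along the line to a target location, provided that location lies within a min and max range.
; PerformAbility sphere-traces from the minimum-range point to the target, ignoring OwningCompass and owner, then passes the hit actor to AffectTarget for damage and finishes.
; CollidesWithEnemies selects the Visibility or Camera trace channel.
; Attack preview shows both range limits as meshes scaled around the owner.
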(fn ConstructionScript
  (|CallParentFunction))

(fn PerformAbility
  (bind (_outhit _bblockinghit) (CallFunction|GetSphereTraceResults))
  (CallFunction|AffectTarget (.HitActor (Collision|BreakHitResult _outhit)) (Math|Vector|SelectVector (.Location (Collision|BreakHitResult _outhit)) (Variables|Default|GetTargetLocation) _bblockinghit))
  (CallFunction|FinishAbility))

(fn AffectTarget
  (params (HitActor :type Actor%20Object%20Reference) (ImpactLocation :type Vector))
  (Game|Damage|ApplyDamage HitActor (Variables|Default|GetDamage) 0 (Components|GetOwner)))

(fn GetSphereTraceResults
  (bind _returnvalue (Components|GetOwner))
  (bind _returnvalue_2 (Transformation|GetActorLocation _returnvalue))
  (bind _output_get (Variables|Default|SetMinRangeLocation (+ (* (Math|Vector|GetForwardVector (Math|Rotator|FindLookatRotation _returnvalue_2 (Variables|Default|GetTargetLocation))) (Variables|Default|GetMinTravelRange)) _returnvalue_2)))
  (bind (_outhit _returnvalue_3) (Collision|SphereTraceByChannel _output_get (Variables|Default|GetTargetLocation) (Variables|Default|GetTravelCollisionRadius) (select (Variables|Default|GetbCollidesWithEnemies) "TraceTypeQuery1" "TraceTypeQuery2") false (Utilities|Array|MakeArray (Variables|Default|GetOwningCompass) (Components|GetOwner)) "None"))
  (return _outhit _returnvalue_3))

(fn CanPerformAttack
  (bind _returnvalue (Components|GetOwner))
  (bind _targetlocation (Variables|Default|GetTargetLocation))
  (bind _returnvalue_2 (Transformation|GetActorLocation _returnvalue))
  (bind _returnvalue_3 (Math|Vector|Distance(Vector) _returnvalue_2 _targetlocation))
  (return (and (>= _returnvalue_3 (Variables|Default|GetMinTravelRange)) (<= _returnvalue_3 (Variables|Default|GetMaxTravelRange)))))

(fn EnableAttackPreview
  (params (bEnabled :type Boolean))
  (|CallParentFunction bEnabled)
  (Rendering|SetVisibility (Variables|Default|GetMinRangePreview) bEnabled false))

(fn PreviewAttack
  (|CallParentFunction)
  (Transformation|SetWorldLocation (Variables|Default|GetMinRangePreview) (Transformation|GetActorLocation (Components|GetOwner)) false true)
  (Transformation|SetRelativeScale3D (Variables|Default|GetMinRangePreview) (Math|Conversions|ToVector(Float) (/ (Variables|Default|GetMinTravelRange) 1e+02)))
  (Transformation|SetRelativeScale3D (Variables|Default|GetMaxRangePreview) (Math|Conversions|ToVector(Float) (/ (Variables|Default|GetMaxTravelRange) 1e+02))))

(fn GetMinRange
  (return (Variables|Default|GetMinTravelRange)))