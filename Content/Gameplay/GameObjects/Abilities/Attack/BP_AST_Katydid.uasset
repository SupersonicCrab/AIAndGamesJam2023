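; Katydid attack ability that throws its target over the owner to the mirrored position on the opposite side.
; CanPerformAttack allows the attack only when the sphere trace hits an actor implementing BPI_TurnActor.
; AffectTarget projects the target's distance to the owner past the owner along the look-at direction, then sets that location instantly without sweep.
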(fn ConstructionScript
  (|CallParentFunction))

(fn AffectTarget
  (params (HitActor :type Actor%20Object%20Reference) (ImpactLocation :type Vector :default "0, 0, 0"))
  (bind _returnvalue (Components|GetOwner))
  (bind _returnvalue_2 (Transformation|GetActorLocation HitActor))
  (bind _returnvalue_3 (Transformation|GetActorLocation _returnvalue))
  (Transformation|SetActorLocation HitActor (+ _returnvalue_3 (* (Math|Vector|GetForwardVector (Math|Rotator|FindLookatRotation _returnvalue_2 _returnvalue_3)) (Math|Vector|Distance(Vector) _returnvalue_2 _returnvalue_3))) false false))

(fn CanPerformAttack
  (bind _outhit (CallFunction|GetSphereTraceResults))
  (return (Utilities|DoesObjectImplementInterface (.HitActor (Collision|BreakHitResult _outhit)) "/Game/Gameplay/Systems/BPI_TurnActor.BPI_TurnActor_C")))