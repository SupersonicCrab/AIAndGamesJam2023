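; BP_DashAbility is a movement ability for a dash, currently only a debug probe that does not move the character.
; PerformAbility casts its owner to Character and sweeps a capsule, sized from the character's capsule component, from its location to Destination on the Visibility channel.
; It draws the trace persistently and prints whether it hit.
; Destination is not set here, and the event graph holds only disabled stubs.
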(event EventBeginPlay
  (|CallParentFunction) ; This node is disabled and will not be called.\nDrag off pins to build functionality.
)

(event Collision|EventActorBeginOverlap
  (params (OtherActor :type Actor%20Object%20Reference))
  (|CallParentFunction OtherActor) ; This node is disabled and will not be called.\nDrag off pins to build functionality.
)

(event EventTick
  (params (DeltaSeconds :type Float%20%28single-precision%29))
  (|CallParentFunction DeltaSeconds) ; This node is disabled and will not be called.\nDrag off pins to build functionality.
)

(fn ConstructionScript
  (|CallParentFunction))

(fn PerformAbility
  (bind _ascharacter (Utilities|Casting|CastToCharacter (Components|GetOwner)))
  (bind _returnvalue (Collision|CapsuleTraceByChannel (Transformation|GetActorLocation _ascharacter) (Variables|Default|GetDestination) (Components|Capsule|GetScaledCapsuleRadius (Variables|/Script/Engine.Character|GetCapsuleComponent _ascharacter)) (Variables|/Script/Engine.CapsuleComponent|GetCapsuleHalfHeight (Variables|/Script/Engine.Character|GetCapsuleComponent _ascharacter)) "TraceTypeQuery1" false 0 "Persistent"))
  (Development|PrintString (Utilities|String|ToString(Boolean) _returnvalue)))