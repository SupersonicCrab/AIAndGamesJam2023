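; Actor component that gives its owner a movement ability, spawned as a separate actor on BeginPlay and destroyed on EndPlay.
; PerformMovementAbility sets the ability's destination at the owner's current Z height, binds to its finish event and starts it.
; When the ability finishes, the component broadcasts OnMovementAbilityFinished, with debug prints at start and finish.
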(event Custom|PerformMovementAbility
  (params (Destination :type Vector))
  (Variables|/Game/Gameplay/GameObjects/Abilities/Movement/BP_MovementAbility.BP_MovementAbility_C|SetDestination (Variables|Default|GetMovementAbility) (Math|Vector|MakeVector (.x Destination) (.y Destination) (.z (Transformation|GetActorLocation (Components|GetOwner)))))
  (Development|PrintString (Utilities|String|Append (Utilities|GetDisplayName (Components|GetOwner)) " starting movement ability " (Utilities|GetDisplayName (Variables|Default|GetMovementAbility))))
  (EventDispatchers|AssignOnAbilityFinished (Variables|Default|GetMovementAbility) (delegate Custom|OnAbilityFinished_Event))
  (Default|PerformAbility (Variables|Default|GetMovementAbility)))

(event Custom|OnAbilityFinished_Event
  (params (Ability :type BP%20Ability%20Object%20Reference))
  (Development|PrintString (Utilities|String|Append (Utilities|GetDisplayName (Components|GetOwner)) " finished movement ability " (Utilities|GetDisplayName Ability)))
  (Default|CallOnMovementAbilityFinished (Variables|Default|GetMovementAbility)))

(event EventBeginPlay
  (CallFunction|CreateMovementAbility (Variables|Default|GetMovementAbilityClass)))

(event EventEndPlay
  (params (EndPlayReason :type EEndPlayReason%20Enum :default "Destroyed"))
  (Actor|DestroyActor (Variables|Default|GetMovementAbility)))

(fn CreateMovementAbility
  (params (Class :type BP%20Movement%20Ability%20Class%20Reference))
  (bind _returnvalue (Game|SpawnActorfromClass Class (Math|Transform|MakeTransform "0, 0, 0" "0, 0, 0" "1.000000,1.000000,1.000000") "Undefined" "MultiplyWithRoot" (Components|GetOwner) 0))
  (Variables|Default|SetMovementAbility _returnvalue))