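; Actor component that tracks an integer health pool for its owner and broadcasts damage, healing and death.
; On BeginPlay it binds to the owner's OnTakeAnyDamage and fills health to maximum.
; TakeDamage subtracts rounded damage with clamping, fires OnTakeDamage, then fires OnDeath on any hit that leaves health at zero.
; Heal adds health up to the maximum and broadcasts the new value through OnHealed.
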(event EventBeginPlay
  (EventDispatchers|AssignOnTakeAnyDamage (Components|GetOwner) (EventDispatchers|CreateEvent :!event TakeDamage))
  (Variables|Default|SetHealth (Variables|Default|GetMaxHealth)))

(fn TakeDamage
  (params (DamagedActor :type Actor%20Object%20Reference) (Damage :type Float%20%28single-precision%29) (DamageType :type Damage%20Type%20Object%20Reference) (InstigatedBy :type Controller%20Object%20Reference) (DamageCauser :type Actor%20Object%20Reference))
  (bind _returnvalue (Math|Float|Round Damage))
  (Variables|Default|SetHealth (Math|Integer|Clamp(Integer) (- (Variables|Default|GetHealth) _returnvalue) 0 (Variables|Default|GetMaxHealth)))
  (Default|CallOnTakeDamage _returnvalue)
  (if (<= (Variables|Default|GetHealth) 0)
    (Default|CallOnDeath)))

(fn Heal
  (params (HealAmount :type Integer))
  (bind _output_get (Variables|Default|SetHealth (Math|Integer|Clamp(Integer) (+ (Variables|Default|GetHealth) HealAmount) 0 (Variables|Default|GetMaxHealth))))
  (Default|CallOnHealed _output_get))