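; BP_Compass is a compass object with sixteen static mesh segments, two per cardinal and intercardinal direction, each representing a selectable or disabled bearing.
; The construction script maps each bearing enum value to its mesh, enabling reverse lookup from mesh to bearing with a fallback value.
; Updating swaps each segment's material and toggles query-only collision according to the DisabledBearing list.
; A helper shows or hides all segments together.
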(fn ConstructionScript
  (CallFunction|AddBearing "NewEnumerator0" (Variables|Default|GetNW1))
  (CallFunction|AddBearing "NewEnumerator1" (Variables|Default|GetNW2))
  (CallFunction|AddBearing "NewEnumerator2" (Variables|Default|GetN1))
  (CallFunction|AddBearing "NewEnumerator3" (Variables|Default|GetN2))
  (CallFunction|AddBearing "NewEnumerator4" (Variables|Default|GetNE1))
  (CallFunction|AddBearing "NewEnumerator5" (Variables|Default|GetNE2))
  (CallFunction|AddBearing "NewEnumerator6" (Variables|Default|GetE1))
  (CallFunction|AddBearing "NewEnumerator7" (Variables|Default|GetE2))
  (CallFunction|AddBearing "NewEnumerator8" (Variables|Default|GetSE1))
  (CallFunction|AddBearing "NewEnumerator9" (Variables|Default|GetSE2))
  (CallFunction|AddBearing "NewEnumerator10" (Variables|Default|GetS1))
  (CallFunction|AddBearing "NewEnumerator11" (Variables|Default|GetS2))
  (CallFunction|AddBearing "NewEnumerator12" (Variables|Default|GetSW1))
  (CallFunction|AddBearing "NewEnumerator13" (Variables|Default|GetSW2))
  (CallFunction|AddBearing "NewEnumerator14" (Variables|Default|GetW1))
  (CallFunction|AddBearing "NewEnumerator15" (Variables|Default|GetW2)))

(fn AddBearing
  (params (CompassBearing :type Enum_CompassBearing%20Enum :default "NewEnumerator0") (StaticMeshComponent :type Static%20Mesh%20Component%20Object%20Reference))
  (Utilities|Map|Add (Variables|Default|GetBearingToMesh) CompassBearing StaticMeshComponent))

(fn IsBearingEnabled
  (params (CompassBearing :type Enum_CompassBearing%20Enum :default "NewEnumerator0"))
  (return (== (Utilities|Array|FindItem (Variables|Default|GetDisabledBearing) CompassBearing) -1)))

(fn UpdateCompassBearings
  (bind _keys (Utilities|Map|Keys (Variables|Default|GetBearingToMesh)))
  (bind _values (Utilities|Map|Values (Variables|Default|GetBearingToMesh)))
  (for (_array_element _array_index) _keys
    (Rendering|Material|SetMaterial (Utilities|Array|Get(acopy) _values _array_index) 0 (select (CallFunction|IsBearingEnabled _array_element) "/Game/Assets/Compass/MI_CompassEnabled.MI_CompassEnabled" "/Game/Assets/Compass/MI_CompassDisabled.MI_CompassDisabled"))
    (Collision|SetCollisionEnabled (Utilities|Array|Get(acopy) _values _array_index) (select (CallFunction|IsBearingEnabled _array_element) "QueryOnly" "NoCollision"))))

(fn GetBearingfromMesh
  (params (BearingMesh :type Static%20Mesh%20Component%20Object%20Reference))
  (bind _values (Utilities|Map|Values (Variables|Default|GetBearingToMesh)))
  (if (== (Utilities|Array|FindItem _values BearingMesh) -1)
    (return "NewEnumerator16")
    (else
      (bind _keys (Utilities|Map|Keys (Variables|Default|GetBearingToMesh)))
      (return (Utilities|Array|Get(acopy) _keys (Utilities|Array|FindItem _values BearingMesh))))))

(fn SetVisibility
  (params (bVisible :type Boolean))
  (Rendering|SetVisibility (Variables|Default|GetW2) bVisible false))